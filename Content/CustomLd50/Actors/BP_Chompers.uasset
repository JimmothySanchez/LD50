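; BP_Chompers is a chomping hazard character that lunges periodically and damages what it touches.
; A timeline drives the UpperJaw rotation, alongside an attached chomp sound started on BeginPlay.
; A looping timer briefly raises walk speed, triggers a jump, then zeroes speed for a burst-and-stop hop; no movement input appears in this graph.
; Any actor that begins overlapping its Box takes damage.
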(event OnComponentBeginOverlap(Box)
  (params (OverlappedComponent :type Primitive%20Component%20Object%20Reference) (OtherActor :type Actor%20Object%20Reference) (OtherComp :type Primitive%20Component%20Object%20Reference) (OtherBodyIndex :type Integer) (bFromSweep :type Boolean) (SweepResult :type Hit%20Result%20Structure%20%28by%20ref%29))
  (Game|Damage|ApplyDamage OtherActor 3.0 0 0))

(event Custom|CustomEvent_0
  (Variables|/Script/Engine.CharacterMovementComponent|SetMaxWalkSpeed (Variables|Character|GetCharacterMovement) 2.4e+03)
  (Utilities|FlowControl|Delay 0.1)
  (Character|Jump)
  (Utilities|FlowControl|Delay 0.5)
  (Variables|/Script/Engine.CharacterMovementComponent|SetMaxWalkSpeed (Variables|Character|GetCharacterMovement) 0.0))

(event EventBeginPlay
  (Utilities|FlowControl|Sequence
    (:then_0
      (bind _newtrack_0 (Timeline|Timeline_0 Play)
        (:Update
          (Transformation|SetRelativeRotation (Variables|Default|GetUpperJaw) (Math|Rotator|Lerp(Rotator) "0, 0, 0" "45.000000, 0, 0" _newtrack_0) false false))))
    (:then_1
      (Utilities|Time|SetTimerbyEvent (delegate Custom|CustomEvent_0) 3.0 true))
    (:then_2
      (bind _returnvalue (Audio|SpawnSoundAttached "/Game/CustomLd50/Audio/Effects/Moncher.Moncher" (Variables|Collision|GetCapsuleComponent) "None" "0, 0, 0" "0, 0, 0" "KeepWorldPosition" false 0.5 1.0 0.0 "/Game/CustomLd50/Audio/CloseAttenuation.CloseAttenuation" "/Game/CustomLd50/Audio/NewSoundConcurrency.NewSoundConcurrency"))
      (Audio|Components|Audio|Play _returnvalue 0.0))))

(event Collision|EventActorBeginOverlap
  (params (OtherActor :type Actor%20Object%20Reference)))

(event EventTick
  (params (DeltaSeconds :type Float%20%28single-precision%29)))

(fn ConstructionScript)