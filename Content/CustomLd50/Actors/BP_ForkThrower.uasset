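; Enemy actor that periodically lobs forks, and after an initial delay knives, at actors tagged "HotDog".
; It picks a random target on BeginPlay and after each fork throw, rotating its eyeballs on Tick from that target's position while a timeline moves its hands.
; Projectiles launch along suggested arcs toward random points around the target, within a box whose size a second timeline drives to vary accuracy.
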(event Custom|ForkThrow
  (CallFunction|ThrowAFork))

(event Custom|ThrowKnife
  (CallFunction|ThrowAKnife))

(event EventBeginPlay
  (CallFunction|ChooseATarget)
  (Utilities|FlowControl|Sequence
    (:then_0
      (bind _newtrack_0 (Timeline|Timeline_0 Play)
        (:Update
          (Transformation|AddLocalOffset (Variables|Default|GetHandR) (* _newtrack_0 3.0) true false)
          (Transformation|AddLocalOffset (Variables|Default|GetHandL) (* _newtrack_0 3.0) true false))))
    (:then_1
      (Utilities|Time|SetTimerbyEvent (delegate Custom|ForkThrow) (Variables|Default|GetThrowCooldown) true))
    (:then_2
      (Utilities|Time|SetTimerbyEvent (delegate Custom|ThrowKnife) 7.0 true 3e+01))
    (:then_3
      (bind _newtrack_0_2 (Timeline|Timeline_1 Play)
        (:Update
          (Variables|Default|SetHitrangeBoxMax (Math|Float|Lerp 1.0 5e+02 _newtrack_0_2)))))))

(event Collision|EventActorBeginOverlap
  (params (OtherActor :type Actor%20Object%20Reference)))

(event EventTick
  (params (DeltaSeconds :type Float%20%28single-precision%29))
  (bind _target (Variables|Default|GetTarget))
  (Utilities|IsValid _target
    (:Is%20Valid
      (Transformation|SetWorldRotation (Variables|Default|GetEyeballR) (Math|Rotator|FindLookatRotation (Transformation|GetActorLocation _target) (Transformation|GetWorldLocation (Variables|Default|GetEyeballR))) false false)
      (Transformation|SetWorldRotation (Variables|Default|GetEyeballL) (Math|Rotator|FindLookatRotation (Transformation|GetActorLocation (Variables|Default|GetTarget)) (Transformation|GetWorldLocation (Variables|Default|GetEyeballL))) false false))))

(fn ConstructionScript)

(fn ChooseATarget
  (bind _outactors (Actor|GetAllActorswithTag "HotDog"))
  (Variables|Default|SetTarget (.OutItem (Utilities|Array|Random _outactors))))

(fn ThrowAFork
  (bind _fork (Variables|Default|GetFork))
  (bind _hitrangeboxmax (Variables|Default|GetHitrangeBoxMax))
  (bind _returnvalue (Transformation|GetWorldLocation _fork))
  (bind _outlaunchvelocity (Game|SuggestProjectileVelocityCustomArc _returnvalue (Math|Random|RandomPointinBoundingBox (Transformation|GetActorLocation (Variables|Default|GetTarget)) (Math|Vector|MakeVector _hitrangeboxmax _hitrangeboxmax _hitrangeboxmax)) 0.0 0.5))
  (bind _returnvalue_2 (Game|SpawnActorfromClass "/Game/CustomLd50/Actors/BP_ForkProjectile.BP_ForkProjectile_C" (Math|Transform|MakeTransform _returnvalue (Math|Conversions|RotationFromXVector _outlaunchvelocity) "1.000000,1.000000,1.000000") "Undefined" 0 0.0 0))
  (Variables|/Script/Engine.MovementComponent|SetVelocity (Variables|/Game/CustomLd50/Actors/BP_ForkProjectile.BP_ForkProjectile_C|GetProjectileMovement _returnvalue_2) _outlaunchvelocity)
  (CallFunction|ChooseATarget))

(fn ThrowAKnife
  (bind _knife (Variables|Default|GetKnife))
  (bind _hitrangeboxmax (Variables|Default|GetHitrangeBoxMax))
  (bind _returnvalue (Transformation|GetWorldLocation _knife))
  (bind _outlaunchvelocity (Game|SuggestProjectileVelocityCustomArc _returnvalue (Math|Random|RandomPointinBoundingBox (Transformation|GetActorLocation (Variables|Default|GetTarget)) (Math|Vector|MakeVector _hitrangeboxmax _hitrangeboxmax _hitrangeboxmax)) 0.0 0.5))
  (bind _returnvalue_2 (Game|SpawnActorfromClass "/Game/CustomLd50/Actors/BP_KnifeProjectile.BP_KnifeProjectile_C" (Math|Transform|MakeTransform _returnvalue (Math|Conversions|RotationFromXVector _outlaunchvelocity) "1.000000,1.000000,1.000000") "Undefined" 0 0.0 0))
  (Variables|/Script/Engine.MovementComponent|SetVelocity (Variables|/Game/CustomLd50/Actors/BP_KnifeProjectile.BP_KnifeProjectile_C|GetProjectileMovement _returnvalue_2) _outlaunchvelocity))